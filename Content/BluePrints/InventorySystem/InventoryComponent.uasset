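; Inventory component that stores item slots and toggles their on-screen window for a player controller.
; ToggleInventory picks a backpack or standard widget by checking InventoryName for "BackPack", then creates or removes it, switching cursor and input mode.
; AddToInventory scans slots in order, stacking onto a same-class item or filling an empty slot, whichever comes first.
; Items finding no slot are silently ignored, as the length-comparison exit never fires.
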(fn `AddToInventory`
  (params (ItemsToAdd :type "/Game/BluePrints/InventorySystem/Items/SlotStructure Structure"))
  (bind (_item _quantity) (break `/Game/BluePrints/InventorySystem/Items/SlotStructure` ItemsToAdd))
  (bind _inventoryslots (`self.InvenTorySlots`))
  (bind (_itemstoadd_item _itemstoadd_quantity) (break `/Game/BluePrints/InventorySystem/Items/SlotStructure` (`local.ItemsToAdd`)))
  (bind _returnvalue (`KismetArrayLibrary.Array_Length` _inventoryslots))
  (for (_array_element _array_index) _inventoryslots
    (bind _item_2 (break `/Game/BluePrints/InventorySystem/Items/SlotStructure` _array_element))
    ;[1 1 1] Check if it is the same item
    (if (== (`.Class_19_F8036CA1454B2F07EDBA4ABFAEBD318E` (break `/Game/BluePrints/InventorySystem/Items/ItemStruct` _item_2)) (`.Class_19_F8036CA1454B2F07EDBA4ABFAEBD318E` (break `/Game/BluePrints/InventorySystem/Items/ItemStruct` (break `/Game/BluePrints/InventorySystem/Items/SlotStructure` (`local.ItemsToAdd`)))))
      (bind (_output_item _output_quantity) (break `/Game/BluePrints/InventorySystem/Items/SlotStructure` (`|GetArrayItem` _inventoryslots _array_index)))
      (`KismetArrayLibrary.Array_Set` _inventoryslots _array_index (make `/Game/BluePrints/InventorySystem/Items/SlotStructure` _item (+ _output_quantity _quantity)))
      (return)
      (elif (== (`.Class_19_F8036CA1454B2F07EDBA4ABFAEBD318E` (break `/Game/BluePrints/InventorySystem/Items/ItemStruct` _item_2)) null)
        (`KismetArrayLibrary.Array_Set` _inventoryslots _array_index (make `/Game/BluePrints/InventorySystem/Items/SlotStructure` _itemstoadd_item _itemstoadd_quantity))
        (return)
        (elif (and (!= (`.Class_19_F8036CA1454B2F07EDBA4ABFAEBD318E` (break `/Game/BluePrints/InventorySystem/Items/ItemStruct` (`.Item_2_44BABA8C49A8909C6902A690A57C9AA5` (break `/Game/BluePrints/InventorySystem/Items/SlotStructure` _array_element)))) (`.Class_19_F8036CA1454B2F07EDBA4ABFAEBD318E` (break `/Game/BluePrints/InventorySystem/Items/ItemStruct` (break `/Game/BluePrints/InventorySystem/Items/SlotStructure` (`local.ItemsToAdd`))))) (> _returnvalue _returnvalue))
          (return))))))

(fn `ToggleInventory`
  (params (PlayerController :type "PlayerController Object Reference"))
  (bind _inventorywindow_ref (`self.InvenToryWindow_ref`))
  (bind _backpackwindow (`self.BackPackWindow`))
  (`/Engine/EditorBlueprintResources/StandardMacros.IsValid` PlayerController
    (:`Is Valid`
      (set `PlayerController.bShowMouseCursor` true PlayerController)
      (`WidgetBlueprintLibrary.SetInputMode_GameAndUIEx` PlayerController null)
      (if (`KismetStringLibrary.Contains` (`KismetTextLibrary.Conv_TextToString` (`self.InventoryName`)) (`KismetTextLibrary.Conv_TextToString` "BackPack"))
        (`/Engine/EditorBlueprintResources/StandardMacros.IsValid` _backpackwindow
          (:`Is Valid`
            (`Widget.RemoveFromParent` _backpackwindow)
            (set `self.BackPackWindow` null)
            (`WidgetBlueprintLibrary.SetInputMode_GameOnly` PlayerController)
            (set `PlayerController.bShowMouseCursor` false PlayerController))
          (:`Is Not Valid`
            (bind _returnvalue (`|CreateWidget` "/Game/BluePrints/InventorySystem/InvenToryUI/BackPackWindow_W.BackPackWindow_W_C" PlayerController (`self.InventoryName`) self))
            (bind _output_get (set `self.BackPackWindow` _returnvalue))
            (`UserWidget.AddToViewport` _output_get 0)))
        (else
          (`/Engine/EditorBlueprintResources/StandardMacros.IsValid` _inventorywindow_ref
            (:`Is Valid`
              (`Widget.RemoveFromParent` _inventorywindow_ref)
              (set `self.InvenToryWindow_ref` null)
              (`WidgetBlueprintLibrary.SetInputMode_GameOnly` PlayerController)
              (set `PlayerController.bShowMouseCursor` false PlayerController))
            (:`Is Not Valid`
              (bind _returnvalue_2 (`|CreateWidget` "/Game/BluePrints/InventorySystem/InvenToryUI/InventoryWindow.InventoryWindow_C" PlayerController (`self.InventoryName`) self))
              (set `self.InvenToryWindow_ref` _returnvalue_2)
              (`UserWidget.AddToViewport` (`self.InvenToryWindow_ref`) 0))))))))