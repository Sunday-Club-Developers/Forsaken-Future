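; Crafting table Blueprint that prompts a nearby player and opens or closes crafting on interaction.
; Entering its Box trigger with a player-controlled pawn shows an on-screen "press E" message widget, removed after a short delay or when a pawn leaves.
; The InterAct event passes the PlayerController to CraftingComponent's ToggleCraftingTable, delegating the crafting behavior to that component.
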(event `self.Box.OnComponentBeginOverlap`
  (params (OverlappedComponent :type "PrimitiveComponent Object Reference") (OtherActor :type "Actor Object Reference") (OtherComp :type "PrimitiveComponent Object Reference") (OtherBodyIndex :type Integer) (bFromSweep :type Boolean) (SweepResult :type "HitResult Structure (by ref)"))
  (bind _scrmessref (`self.ScrMessRef`))
  ;[0.02363 1 0] Handle Whyen player comes near
  (bind _aspawn (cast `Pawn` OtherActor))
  (bind _asplayer_controller (cast `PlayerController` (`Pawn.GetController` _aspawn)))
  (`/Engine/EditorBlueprintResources/StandardMacros.IsValid` (`self.ScrMessRef`)
    (:`Is Valid`
      _)
    (:`Is Not Valid`
      (bind _returnvalue (`|CreateWidget` "/Game/BluePrints/InventorySystem/Items/ItemUi/ItemScreenmessage.ItemScreenmessage_C" _asplayer_controller "CraftingTabel, press 'E' To Interact"))
      (set `self.ScrMessRef` _returnvalue)))
  (`UserWidget.AddToViewport` (`self.ScrMessRef`) 0)
  (`KismetSystemLibrary.Delay` 1.0)
  (`/Engine/EditorBlueprintResources/StandardMacros.IsValid` _scrmessref
    (:`Is Valid`
      (`Widget.RemoveFromParent` _scrmessref)
      (set `self.ScrMessRef` null))))

(event `self.Box.OnComponentEndOverlap`
  (params (OverlappedComponent :type "PrimitiveComponent Object Reference") (OtherActor :type "Actor Object Reference") (OtherComp :type "PrimitiveComponent Object Reference") (OtherBodyIndex :type Integer))
  (bind _scrmessref (`self.ScrMessRef`))
  ;[0.02363 1 0] Handle Whyen player comes near
  (cast `Pawn` OtherActor)
  (`/Engine/EditorBlueprintResources/StandardMacros.IsValid` _scrmessref
    (:`Is Valid`
      (`Widget.RemoveFromParent` _scrmessref)
      (set `self.ScrMessRef` null))))

(event `/Game/BluePrints/InventorySystem/Items/InterActInterFace.InterAct`
  (params (PlayerController :type "PlayerController Object Reference") (PlayerCharacter :type "/Game/BluePrints/CharactersBP/Base_Character Object Reference"))
  (`/Engine/EditorBlueprintResources/StandardMacros.IsValid` PlayerController
    (:`Is Valid`
      (`/Game/BluePrints/CraftingSystem/CraftingComponent.ToggleCraftingTable` (`self.CraftingComponent`) PlayerController))))

(fn `UserConstructionScript`)